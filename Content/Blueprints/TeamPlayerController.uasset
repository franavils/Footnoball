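; Player controller for a team of third-person characters that one player cycles through with the Pass / Swap Player input.
; Shortly after BeginPlay it builds a roster from the controlled pawn and its two linked teammates, stamping each with the player index.
; Swapping possesses the character at the current index, then advances it with wraparound.
; Events append new characters and, after a short delay, prune invalid entries.
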(event `self.ReceiveBeginPlay`
  (`KismetSystemLibrary.Delay` 0.5)
  (bind _asthird_person_character (cast `/Game/ThirdPersonBP/Blueprints/ThirdPersonCharacter` (`self.K2_GetPawn` (`GameplayStatics.GetPlayerController` (`self.PlayerInt`)))))
  (set `self.Character1` _asthird_person_character)
  (set `self.Character2` (`/Game/ThirdPersonBP/Blueprints/ThirdPersonCharacter.Character2` _asthird_person_character))
  (set `self.Character3` (`/Game/ThirdPersonBP/Blueprints/ThirdPersonCharacter.Character3` _asthird_person_character))
  (bind _output_get (set `self.Characters` (`|MakeArray` (`self.Character1`) (`self.Character2`) (`self.Character3`))))
  (for _array_element _output_get
    (bind _asthird_person_character_2 (cast `/Game/ThirdPersonBP/Blueprints/ThirdPersonCharacter` _array_element))
    (set `/Game/ThirdPersonBP/Blueprints/ThirdPersonCharacter.PlayerInt` (`self.PlayerInt`) _asthird_person_character_2)))

(event `New Character`
  (params (Character :type "/Game/ThirdPersonBP/Blueprints/ThirdPersonCharacter Object Reference"))
  (`KismetArrayLibrary.Array_Add` (`self.Characters`) Character))

(event `RemoveEmpty`
  (`KismetSystemLibrary.Delay` 0.2)
  (for (_array_element _array_index) (`self.Characters`)
    (if (not (`KismetSystemLibrary.IsValid` _array_element))
      (`KismetArrayLibrary.Array_Remove` (`self.Characters`) _array_index))))

(event `Swap Player`
  (`self.Possess` (`|GetArrayItem` (`self.Characters`) (`self.CurrentArrayIndex`)))
  (if (>= (`self.CurrentArrayIndex`) (`KismetArrayLibrary.Array_LastIndex` (`self.Characters`)))
    (set `self.CurrentArrayIndex` 0)
    (else
      (set `self.CurrentArrayIndex` (+ (`self.CurrentArrayIndex`) 1)))))

(event `InputAction|Pass / Swap Player`
  (params (Key :type "Key Structure"))
  (:`Pressed`
    (`self.Swap Player`)))

(fn `UserConstructionScript`)