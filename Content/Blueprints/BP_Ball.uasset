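; BP_Ball is a pickup ball that a ThirdPersonCharacter collects by walking into it.
; When BallSphere begins overlapping a character that does not already have a ball, it calls GetBall on that character and destroys itself.
; A character already holding a ball leaves it in place, and debug prints report each case.
; A debug sphere draw for BallSphere is present but never runs.
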(event `self.ReceiveBeginPlay`)

(event `self.ReceiveTick`
  (params (DeltaSeconds :type "Float (single-precision)")))

(event `self.Ball Sphere.OnComponentBeginOverlap`
  (params (OverlappedComponent :type "PrimitiveComponent Object Reference") (OtherActor :type "Actor Object Reference") (OtherComp :type "PrimitiveComponent Object Reference") (OtherBodyIndex :type Integer) (bFromSweep :type Boolean) (SweepResult :type "HitResult Structure (by ref)"))
  (`KismetSystemLibrary.PrintString` "Ball collided")
  (bind _asthird_person_character (cast `/Game/ThirdPersonBP/Blueprints/ThirdPersonCharacter` OtherActor))
  (if (`/Game/ThirdPersonBP/Blueprints/ThirdPersonCharacter.HasBall` _asthird_person_character)
    (`KismetSystemLibrary.PrintString` "Player has ball" true true (struct :`G` 1.0 :`B` 0.390673 :`A` 1.0))
    (else
      (`KismetSystemLibrary.PrintString` "Second collision" true true (struct :`R` 1.0 :`G` 0.029223 :`A` 1.0))
      (`/Game/ThirdPersonBP/Blueprints/ThirdPersonCharacter.GetBall` _asthird_person_character)
      (`self.K2_DestroyActor`))))

(fn `UserConstructionScript`)